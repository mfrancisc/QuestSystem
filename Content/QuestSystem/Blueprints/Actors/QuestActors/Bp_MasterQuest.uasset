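; Base quest actor that tracks which sub-goals from its quest info are currently active.
; Setup copies the starting sub-goal indices into the current indices, then rebuilds the current goal list from them.
; GoToNextSubGoal returns false when no higher index remains, but its logic to advance to the next index is unwired and never runs.
; Event graph and construction script are empty.
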(event EventBeginPlay)

(event Collision|EventActorBeginOverlap
  (params (OtherActor :type Actor%20Object%20Reference)))

(event EventTick
  (params (DeltaSeconds :type Float%20%28single-precision%29)))

(fn ConstructionScript)

(fn UpdateSubGoals
  (Utilities|Array|Clear (Variables|Donottouch!|GetCurrentGoals))
  (for _array_element (Variables|Donottouch!|GetCurrentGoalIndices)
    (Utilities|Array|Add (Variables|Donottouch!|GetCurrentGoals) (Utilities|Array|Get(acopy) (.SubGoals (Utilities|Struct|Breaks_QuestInfo (Variables|QuestInformation|GetQuestInfo))) _array_element)))
  (return))

(fn SetupStartingGoals
  (Utilities|Array|Clear (Variables|Donottouch!|GetCurrentGoalIndices))
  (Variables|Donottouch!|SetCurrentGoalIndices (Variables|QuestInformation|GetStartingSubGoalIndices))
  (CallFunction|UpdateSubGoals)
  (return))

(fn GotoNextSubGoal
  (if (not (<= (+ (.MaxValue (Math|Integer|MaxOfIntArray (Variables|Donottouch!|GetCurrentGoalIndices))) 1) (Utilities|Array|LastIndex (.SubGoals (Utilities|Struct|Breaks_QuestInfo (Variables|QuestInformation|GetQuestInfo))))))
    (return false)))